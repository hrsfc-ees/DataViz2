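; Hand pawn that visualizes voltage readings from a socket on a dynamic material and lets the user lay out the sensors.
; Each tick writes the voltage array into indexed material scalar parameters.
; In edit mode, a SensorSelector widget is shown, and a grabbed sensor follows the cursor over the hand via trace-derived collision UVs until left-click.
; Events also set per-sensor radius and a shared offset on the material.
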(event `self.ReceiveTick`
  (params (DeltaSeconds :type "Float (single-precision)"))
  (bind _hitresult (`PlayerController.GetHitResultUnderCursorByChannel` (`GameplayStatics.GetPlayerController` 0) "TraceTypeQuery1" false))
  (bind (_bblockinghit _binitialoverlap _time _distance _location) (`GameplayStatics.BreakHitResult` _hitresult))
  ;[1 1 1] Every time the game updates
  (`|ExecutionSequence`
    (:`then_0`
      ;[1 1 1] Custom function that returns values from socket
      (bind (_voltagearray _returnvalue) (`self.GetVoltage`))
      (if _returnvalue
        (for (_array_element _array_index) _voltagearray
          ;[1 1 1] Set Values On Material
          (`MaterialInstanceDynamic.SetScalarParameterValue` (`self.FTCInstance_M`) (`KismetStringLibrary.Conv_StringToName` (`KismetStringLibrary.Concat_StrStr` "Density" (`KismetStringLibrary.Conv_IntToString` _array_index))) _array_element))))
    (:`then_1`
      ;[1 1 1] Changing Position
      (if (and (`self.Editing?`) (`self.Grabbed?`))
        (cast `/Game/HandPawn/HandPawn_BP` (`.HitActor` (`GameplayStatics.BreakHitResult` _hitresult)))
        (bind (_outhit _returnvalue_2) (`KismetSystemLibrary.LineTraceSingle` :`Start` (+ _location (0.0 0.0 100.0)) :`End` (+ _location (0.0 0.0 -50.0)) :`TraceChannel` "TraceTypeQuery1" :`bTraceComplex` true :`bIgnoreSelf` false))
        (if _returnvalue_2
          (bind _uv (`GameplayStatics.FindCollisionUV` _outhit))
          (`MaterialInstanceDynamic.SetVectorParameterValue` (`self.FTCInstance_M`) (`KismetStringLibrary.Conv_StringToName` (`KismetStringLibrary.Concat_StrStr` "Location" (`KismetStringLibrary.Conv_IntToString` (`self.CurrSensor`)))) (make `LinearColor` (`KismetMathLibrary.BreakVector2D` _uv) (`.Y` (`KismetMathLibrary.BreakVector2D` _uv)) 0.0 1.0)))))))

(event `Key|LeftMouseButton`
  (params (Key :type "Key Structure"))
  (:`Pressed`
    (set `self.Grabbed?` false)))

(event `Key|R`
  (params (Key :type "Key Structure"))
  (:`Pressed`
    (`self.ClearQueue`)))

(event `SetSensor`
  (params (SensorNo :type Integer))
  (set `self.CurrSensor` SensorNo)
  (set `self.Grabbed?` true))

(event `self.ReceiveBeginPlay`
  (bind _returnvalue (`GameplayStatics.GetPlayerController` 0))
  (`WidgetBlueprintLibrary.SetInputMode_GameOnly` _returnvalue)
  (set `PlayerController.bShowMouseCursor` false _returnvalue)
  (bind _returnvalue_2 (`|CreateWidget` "/Game/UI/SensorSelector.SensorSelector_C" _returnvalue))
  (set `self.SensorSelectorref` _returnvalue_2))

(event `InputAction|Edit`
  (params (Key :type "Key Structure"))
  (bind _returnvalue (`GameplayStatics.GetPlayerController` 0))
  (bind _sensorselectorref (`self.SensorSelectorref`))
  (:`Pressed`
    (set `PlayerController.bShowMouseCursor` true _returnvalue)
    (`UserWidget.AddToViewport` _sensorselectorref 0)
    (`WidgetBlueprintLibrary.SetInputMode_GameAndUIEx` _returnvalue _sensorselectorref "LockAlways" false)
    (set `self.Editing?` true)))

(event `InputAction|StopEdit`
  (params (Key :type "Key Structure"))
  (bind _returnvalue (`GameplayStatics.GetPlayerController` 0))
  (:`Pressed`
    (`WidgetBlueprintLibrary.SetInputMode_GameOnly` _returnvalue)
    (set `PlayerController.bShowMouseCursor` false _returnvalue)
    (`Widget.RemoveFromParent` (`self.SensorSelectorref`))
    (set `self.Editing?` false)))

(event `SetRadius`
  (params (Radius :type "Float (double-precision)"))
  (`MaterialInstanceDynamic.SetScalarParameterValue` (`self.FTCInstance_M`) (`KismetStringLibrary.Conv_StringToName` (`KismetStringLibrary.Concat_StrStr` "Radius" (`KismetStringLibrary.Conv_IntToString` (`self.CurrSensor`)))) Radius))

(event `SetOffset`
  (params (Offset :type "Float (double-precision)"))
  (`KismetSystemLibrary.PrintString` (`KismetStringLibrary.Conv_DoubleToString` Offset))
  (`MaterialInstanceDynamic.SetScalarParameterValue` (`self.FTCInstance_M`) "Offset" Offset))

(fn `UserConstructionScript`)